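; Editor-style pawn for placing BP_Spawned objects under the mouse cursor and saving or reloading the layout.
; Keys 1 and 2 choose the class; left click spawns it unless a box overlap finds one there.
; Each placement's class and transform is recorded in a BP_SaveMap, saved with 9.
; Key 0 destroys existing objects, with a delayed respawn from the save inside that destroy loop.
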(event EventBeginPlay
  (Variables|/Script/Engine.PlayerController|SetbShowMouseCursor (Game|GetPlayerController 0) true)
  (bind _returnvalue (SaveGame|CreateSaveGameObject "/Game/Blueprints/BP_SaveMap.BP_SaveMap_C"))
  (Variables|Default|SetLevelInfo _returnvalue))

(event Input|MouseEvents|LeftMouseButton
  (params (Key :type Key%20Structure :default "AnyKey"))
  (bind _returnvalue (Game|GetPlayerController 0))
  (bind _spawnoffset (Variables|Default|GetSpawnOffset))
  (bind _hitresult (Game|Player|GetHitResultUnderCursorbyChannel _returnvalue "TraceTypeQuery1" true))
  (bind _returnvalue_2 (+ (.location _hitresult) _spawnoffset))
  (:Pressed
    (bind _outactors (Collision|BoxOverlapActors _returnvalue_2 "50.000000,50.000000,50.000000" (Variables|Default|GetAllObjectTypes) "/Game/Blueprints/BP_Spawned.BP_Spawned_C" :!class /Script/Engine.KismetSystemLibrary))
    (if (not (> (Utilities|Array|Length _outactors) 0))
      (bind _returnvalue_3 (Game|SpawnActorfromClass (Variables|Default|GetCurrentSpawnedClass) (Math|Transform|MakeTransform _returnvalue_2 "0, 0, 0" "1,1,1") "Undefined" 0 0))
      (Utilities|Array|Add (Variables|/Game/Blueprints/BP_SaveMap.BP_SaveMap_C|GetSavedObjectPlacements (Variables|Default|GetLevelInfo)) (Utilities|Struct|MakeSavedObjectPlacement (Utilities|GetClass _returnvalue_3) (Transformation|GetActorTransform _returnvalue_3))))))

(event Input|KeyboardEvents|1
  (params (Key :type Key%20Structure :default "AnyKey"))
  (:Pressed
    (Variables|Default|SetCurrentSpawnedClass "/Game/Blueprints/BP_SpawnedChild1.BP_SpawnedChild1_C")))

(event Input|KeyboardEvents|2
  (params (Key :type Key%20Structure :default "AnyKey"))
  (:Pressed
    (Variables|Default|SetCurrentSpawnedClass "/Game/Blueprints/BP_SpawnedChild2.BP_SpawnedChild2_C")))

(event Input|KeyboardEvents|0
  (params (Key :type Key%20Structure :default "AnyKey"))
  (:Pressed
    (bind _returnvalue (SaveGame|LoadGamefromSlot "aa"))
    (bind _outactors (Actor|GetAllActorsOfClass "/Game/Blueprints/BP_Spawned.BP_Spawned_C"))
    (for _array_element _outactors
      (Actor|DestroyActor _array_element)
      (Utilities|FlowControl|Delay 2.0)
      (bind _asbp_save_map (Utilities|Casting|CastToBP_SaveMap _returnvalue))
      (for _array_element_2 (Variables|/Game/Blueprints/BP_SaveMap.BP_SaveMap_C|GetSavedObjectPlacements _asbp_save_map)
        (Game|SpawnActorfromClass (.class _array_element_2) (.transform _array_element_2) "Undefined" 0 0)))))

(event Input|KeyboardEvents|9
  (params (Key :type Key%20Structure :default "AnyKey"))
  (:Pressed
    (SaveGame|SaveGametoSlot (Variables|Default|GetLevelInfo) "aa")))

(fn ConstructionScript)